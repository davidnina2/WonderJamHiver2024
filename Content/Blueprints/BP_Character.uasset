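; Playable Paper2D flipbook character for a versus game, with movement, melee attack and potion use driven by Enhanced Input.
; A Stats map scales movement and drives combat, and movement input and attacks swap directional flipbooks.
; AttackRange overlaps track one target, which attacks damage by attack minus defense and knock back, followed by a short cooldown.
; A lethal hit instead awards a point to the attacker's Index through BP_GameInstanceGenWarf.
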(event OnComponentBeginOverlap(AttackRange)
  (params (OverlappedComponent :type Primitive%20Component%20Object%20Reference) (OtherActor :type Actor%20Object%20Reference) (OtherComp :type Primitive%20Component%20Object%20Reference) (OtherBodyIndex :type Integer) (bFromSweep :type Boolean) (SweepResult :type Hit%20Result%20Structure%20%28by%20ref%29))
  ;[1 1 1] Detect if a layer is within range
  (if (== (Utilities|GetClass OtherActor) "BP_Character_C")
    (Variables|Default|SetActorInRange OtherActor)))

(event OnComponentEndOverlap(AttackRange)
  (params (OverlappedComponent :type Primitive%20Component%20Object%20Reference) (OtherActor :type Actor%20Object%20Reference) (OtherComp :type Primitive%20Component%20Object%20Reference) (OtherBodyIndex :type Integer))
  ;[1 1 1] Detect if a layer is within range
  (if (== (Utilities|GetClass OtherActor) "BP_Character_C")
    (Variables|Default|SetActorInRange 0)))

(event Custom|Update%20Speed
  (bind _charactermovement (Variables|Character|GetCharacterMovement))
  ;[1 1 1] Use potions
  (Variables|/Script/Engine.CharacterMovementComponent|SetMaxWalkSpeed _charactermovement (* (Variables|/Script/Engine.CharacterMovementComponent|GetMaxWalkSpeed _charactermovement) (.Value (Utilities|Map|Find (Variables|Default|GetStats) "(TagName=\"stats.speed\")")))))

(event Input|EnhancedActionEvents|EnhancedInputActionIA_MoveLeftRight
  (params (ActionValue :type Float%20%28double-precision%29) (ElapsedSeconds :type Float%20%28double-precision%29) (TriggeredSeconds :type Float%20%28double-precision%29) (InputAction :type Input%20Action%20Object%20Reference :default "/Game/Blueprints/Controller/Inputs/IA_MoveLeftRight.IA_MoveLeftRight"))
  (bind _sprite (Variables|Default|GetSprite))
  (bind _returnvalue (Class|PaperFlipbookComponent|GetFlipbook _sprite))
  ;[1 1 1] Movement
  (:Triggered
    (Pawn|Input|AddMovementInput (* (Math|Vector|GetRightVector (Math|Rotator|MakeRotator (.Yaw (Math|Rotator|BreakRotator (Pawn|GetControlRotation :!class /Script/Engine.Pawn))) 0.0 0.0)) (.Value (Utilities|Map|Find (Variables|Default|GetStats) "(TagName=\"stats.speed\")"))) ActionValue false)
    (if (!= _returnvalue "/Game/Animations/PFB_AttackLeft.PFB_AttackLeft")
      (if (!= _returnvalue "/Game/Animations/PFB_AttackRight.PFB_AttackRight")
        (CallFunction|UpdateAnimations ActionValue))))
  (:Completed
    (Sprite|SetFlipbook (Variables|Default|GetSprite) "/Game/Animations/PFB_Idle.PFB_Idle")))

(event Input|EnhancedActionEvents|EnhancedInputActionIA_MoveUpDown
  (params (ActionValue :type Float%20%28double-precision%29) (ElapsedSeconds :type Float%20%28double-precision%29) (TriggeredSeconds :type Float%20%28double-precision%29) (InputAction :type Input%20Action%20Object%20Reference :default "/Game/Blueprints/Controller/Inputs/IA_MoveUpDown.IA_MoveUpDown"))
  ;[1 1 1] Movement
  (:Triggered
    (Pawn|Input|AddMovementInput (* (Math|Vector|GetForwardVector (Math|Rotator|MakeRotator (.Yaw (Math|Rotator|BreakRotator (Pawn|GetControlRotation :!class /Script/Engine.Pawn))) 0.0 0.0)) (.Value (Utilities|Map|Find (Variables|Default|GetStats) "(TagName=\"stats.speed\")"))) ActionValue false)
    (if (== (Class|PaperFlipbookComponent|GetFlipbook (Variables|Default|GetSprite)) "/Game/Animations/PFB_Idle.PFB_Idle")
      (CallFunction|UpdateAnimationUpDown ActionValue)))
  (:Completed
    (Sprite|SetFlipbook (Variables|Default|GetSprite) "/Game/Animations/PFB_Idle.PFB_Idle")))

(event Input|EnhancedActionEvents|EnhancedInputActionIA_Attack
  (params (ActionValue :type Boolean) (ElapsedSeconds :type Float%20%28double-precision%29) (TriggeredSeconds :type Float%20%28double-precision%29) (InputAction :type Input%20Action%20Object%20Reference :default "/Game/Blueprints/Controller/Inputs/IA_Attack.IA_Attack"))
  (bind _returnvalue (Transformation|GetActorLocation))
  (bind _sprite (Variables|Default|GetSprite))
  ;[1 1 1] Attack function
  (:Started
    (if (Variables|Default|GetCanIAttack)
      (if (!= (Variables|Default|GetActorInRange) 0)
        (bind _asbp_character (Utilities|Casting|CastToBP_Character (Variables|Default|GetActorInRange)))
        (if (> (- (.Value (Utilities|Map|Find (Variables|BP_Character_C|GetStats _asbp_character) "(TagName=\"stats.health\")")) (Math|Float|Clamp(Float) (- (.Value (Utilities|Map|Find (Variables|Default|GetStats) "(TagName=\"stats.attack\")")) (.Value (Utilities|Map|Find (Variables|BP_Character_C|GetStats _asbp_character) "(TagName=\"stats.defense\")"))) 0.0 1e+09)) 0.0)
          (Utilities|Map|Add (Variables|BP_Character_C|GetStats _asbp_character) "(TagName=\"stats.health\")" (- (.Value (Utilities|Map|Find (Variables|BP_Character_C|GetStats _asbp_character) "(TagName=\"stats.health\")")) (Math|Float|Clamp(Float) (- (.Value (Utilities|Map|Find (Variables|Default|GetStats) "(TagName=\"stats.attack\")")) (.Value (Utilities|Map|Find (Variables|BP_Character_C|GetStats _asbp_character) "(TagName=\"stats.defense\")"))) 0.0 1e+09)))
          (Development|PrintString (Utilities|String|ToString(Float) (- (.Value (Utilities|Map|Find (Variables|BP_Character_C|GetStats _asbp_character) "(TagName=\"stats.health\")")) (Math|Float|Clamp(Float) (- (.Value (Utilities|Map|Find (Variables|Default|GetStats) "(TagName=\"stats.attack\")")) (.Value (Utilities|Map|Find (Variables|BP_Character_C|GetStats _asbp_character) "(TagName=\"stats.defense\")"))) 0.0 1e+09))))
          (if (< (.Y (Math|Vector|BreakVector (Transformation|GetActorLocation _asbp_character))) (.Y (Math|Vector|BreakVector _returnvalue)))
            (Development|PrintString "right")
            (Sprite|SetFlipbook _sprite "/Game/Animations/PFB_AttackRight.PFB_AttackRight")
            (else
              (Development|PrintString "2")
              (Sprite|SetFlipbook _sprite "/Game/Animations/PFB_AttackLeft.PFB_AttackLeft")))
          (Character|LaunchCharacter _asbp_character (* (Math|Vector|GetForwardVector (Math|Rotator|FindLookatRotation _returnvalue (Transformation|GetActorLocation _asbp_character))) 1e+03 (.Value (Utilities|Map|Find (Variables|Default|GetStats) "(TagName=\"stats.knockback\")"))) false false)
          (Variables|Default|SetCanIAttack false)
          (Utilities|FlowControl|Delay 0.5)
          (Variables|Default|SetCanIAttack true)
          (Sprite|SetFlipbook (Variables|Default|GetSprite) "/Game/Animations/PFB_Idle.PFB_Idle")
          (else
            ;;[1 1 1] Set points
            (bind _asbp_game_instance_gen_warf (Utilities|Casting|CastToBP_GameInstanceGenWarf (Game|GetGameInstance)))
            (Default|AddPointtoWinner _asbp_game_instance_gen_warf (Variables|Default|GetIndex))))))))

(event Input|EnhancedActionEvents|EnhancedInputActionIA_UsePotion
  (params (ActionValue :type Boolean) (ElapsedSeconds :type Float%20%28double-precision%29) (TriggeredSeconds :type Float%20%28double-precision%29) (InputAction :type Input%20Action%20Object%20Reference :default "/Game/Blueprints/Controller/Inputs/IA_UsePotion.IA_UsePotion"))
  ;[1 1 1] Use potions
  (if (Utilities|IsValid (Variables|Default|GetPotion))
    (Default|Consume (Variables|Default|GetPotion) self)
    (CallFunction|UpdateSpeed)))

(event EventBeginPlay
  (CallFunction|UpdateSpeed)
  (Sprite|SetFlipbook (Variables|Default|GetSprite) "/Game/Animations/PFB_Idle.PFB_Idle"))

(fn ConstructionScript)

(fn UpdateAnimations
  (params (value :type Float%20%28double-precision%29))
  (bind _sprite (Variables|Default|GetSprite))
  (if (> value 0.0)
    (Sprite|SetFlipbook _sprite "/Game/Animations/PFB_MoveLeft.PFB_MoveLeft")
    (else
      (Sprite|SetFlipbook _sprite "/Game/Animations/PFB_MoveRight.PFB_MoveRight"))))

(fn UpdateAnimationUpDown
  (params (Value :type Float%20%28double-precision%29))
  (bind _sprite (Variables|Default|GetSprite))
  (if (> Value 0.0)
    (Sprite|SetFlipbook _sprite "/Game/Animations/PFB_MoveUp.PFB_MoveUp")
    (else
      (Sprite|SetFlipbook _sprite "/Game/Animations/PFB_MoveDown.PFB_MoveDown"))))