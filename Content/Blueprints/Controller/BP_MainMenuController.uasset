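; Main menu player controller that sets up Enhanced Input and opens the pause menu.
; On BeginPlay it adds the MC_MainMenu mapping context to the local player's input subsystem.
; The IA_Pause action creates a new WBP_PauseMenu widget, adds it to the viewport and pauses the game.
; A separate SetupInput function, not called within this Blueprint, adds MC_MappingCustom and prints debug strings.
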(event Input|EnhancedActionEvents|EnhancedInputActionIA_Pause
  (params (ActionValue :type Boolean) (ElapsedSeconds :type Float%20%28double-precision%29) (TriggeredSeconds :type Float%20%28double-precision%29) (InputAction :type Input%20Action%20Object%20Reference :default "/Game/Blueprints/Controller/Inputs/IA_Pause.IA_Pause"))
  (:Started
    (bind _returnvalue (UserInterface|CreateWidget "/Game/Widgets/WBP_PauseMenu.WBP_PauseMenu_C"))
    (UserInterface|Viewport|AddtoViewport _returnvalue 0)
    (Game|SetGamePaused true)))

(event EventBeginPlay
  (bind _returnvalue (PlayerController|LocalPlayerSubsystems|GetEnhancedInputLocalPlayerSubsystem))
  ;[0.05098 0.05098 0.05098] Add Mapping Context
  (Utilities|IsValid _returnvalue
    (:Is%20Valid
      (Input|AddMappingContext _returnvalue "/Game/Blueprints/Controller/Inputs/MC_MainMenu.MC_MainMenu" 0 "(bIgnoreAllPressedKeysUntilRelease=True,bForceImmediately=False,bNotifyUserSettings=False)"))))

(fn ConstructionScript)

(fn SetupInput
  (bind _returnvalue (PlayerController|LocalPlayerSubsystems|GetEnhancedInputLocalPlayerSubsystem))
  (Utilities|IsValid _returnvalue
    (:Is%20Valid
      (Input|AddMappingContext _returnvalue "/Game/Blueprints/Controller/Inputs/MC_MappingCustom.MC_MappingCustom" 0 "(bIgnoreAllPressedKeysUntilRelease=True,bForceImmediately=False,bNotifyUserSettings=False)")
      (Development|PrintString "Hello"))
    (:Is%20Not%20Valid
      (Development|PrintString "2"))))