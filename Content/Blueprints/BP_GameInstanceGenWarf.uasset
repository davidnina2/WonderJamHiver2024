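; GameInstance Blueprint that keeps the score for a two-player match and ends it when either player wins.
; AddPointToWinner adds a point to Player 1 for winner index 0, otherwise to Player 2.
; When a score reaches seven, it stores the winner's name in WinnerText, shows the WBP_EndGamePanel widget and pauses the game.
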(fn AddPointtoWinner
  (params (WinnerIndex :type Integer))
  (if (== WinnerIndex 0)
    (bind _output_get (Variables|Default|SetPlayer1Points (+ (Variables|Default|GetPlayer1Points) 1)))
    (if (== _output_get 7)
      (Variables|Default|SetWinnerText "Player 1")
      (bind _returnvalue (UserInterface|CreateWidget "/Game/Widgets/WBP_EndGamePanel.WBP_EndGamePanel_C" :!label _label))
      (UserInterface|Viewport|AddtoViewport _returnvalue 0)
      (Game|SetGamePaused true))
    (else
      (bind _output_get_2 (Variables|Default|SetPlayer2Points (+ (Variables|Default|GetPlayer2Points) 1)))
      (if (== _output_get_2 7)
        (Variables|Default|SetWinnerText "Player 2")
        (goto _label)))))