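; Game mode for local multiplayer that creates a controller and character per PlayerStart, spawns timed potions and runs recurring disarm events.
; Looping timers use intervals randomized once at BeginPlay; each event spawns two BP_EventDisarm actors and starts a HUD countdown.
; At zero, disarm actors with a valid Character are destroyed, while one without fails the event and opens LVL_Lab.
; Health and potion updates are forwarded to the HUD.
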(event Custom|HealthUpdated
  (Default|HealthUpdated (Variables|Default|GetHUDWidget)))

(event Custom|OnUpdateEventCountdown
  (bind _result (Math|Float|DecrementFloat (Variables|Default|GetEventTimeRemaining))
    (:%20%20
      (Default|OnEventCountdownUpdated (Variables|Default|GetHUDWidget) _result)
      (if (== _result 0.0)
        (Variables|Default|SetIsEventInProgress false)
        (Utilities|Time|ClearandInvalidateTimerbyHandle (Variables|Default|GetTimerHandle))
        (Default|SetCountdownVisibility (Variables|Default|GetHUDWidget) false)
        (bind _outactors (Actor|GetAllActorsOfClass "/Game/Blueprints/BP_EventDisarm.BP_EventDisarm_C"))
        (bind _array_element (Utilities|Array|ForEachLoopwithBreak _outactors :!label _label)
          (:LoopBody
            (bind _output_get (Variables|Default|SetIsEventSucceeded (Utilities|IsValid (Variables|/Game/Blueprints/BP_EventDisarm.BP_EventDisarm_C|GetCharacter _array_element))))
            (if _output_get
              (Actor|DestroyActor _array_element)
              (else
                (goto _label Break))))
          (:Completed
            (if (Variables|Default|GetIsEventSucceeded)
              (Development|PrintString "s u c c e e d")
              (else
                (CallFunction|OnEventFailed)))))))))

(event Custom|OnRandomEventStarted
  (if (not (Variables|Default|GetIsEventInProgress))
    (Variables|Default|SetIsEventInProgress true)
    (Utilities|Time|SetTimerbyEvent (delegate Custom|OnUpdateEventCountdown) 1.0 true)
    (CallFunction|StartEvent)
    (Development|PrintString "AFTER START EVENT")))

(event Custom|OnEventFailed
  (Development|PrintString "EventFailed")
  (Utilities|FlowControl|Delay 0.2)
  (Game|OpenLevel(byName) "LVL_Lab"))

(event Custom|PotionsUpdated
  (Default|PotionsUpdated (Variables|Default|GetHUDWidget)))

(event EventBeginPlay
  (bind _maxtimeforevent (Variables|Default|GetMaxTimeForEvent))
  (bind _mintimeforevent (Variables|Default|GetMinTimeForEvent))
  (bind _returnvalue (Math|Random|RandomFloatinRange _mintimeforevent _maxtimeforevent))
  (CallFunction|SpawnPlayers)
  (Utilities|Time|SetTimerbyEvent (delegate Custom|OnRandomEventStarted) _returnvalue true)
  (Development|PrintString (Utilities|String|ToString(Float) _returnvalue))
  (Utilities|Time|SetTimerbyFunctionName 0 "SpawnPotion" (Math|Random|RandomFloatinRange 15.0 2e+01) true))

(fn ConstructionScript)

(fn StartEvent
  (bind _hudwidget (Variables|Default|GetHUDWidget))
  (bind _output_get (Variables|Default|SetEventTimeRemaining 1e+01))
  (Default|SetCountdownVisibility _hudwidget true)
  (Default|OnEventCountdownUpdated _hudwidget _output_get)
  (Game|SpawnActorfromClass "/Game/Blueprints/BP_EventDisarm.BP_EventDisarm_C" (Math|Transform|MakeTransform (Math|Random|RandomPointinBoundingBox "0.000000,0.000000,80.000000" "1000.000000,1000.000000,0.000000") "0, 0, 0" "1.000000,1.000000,1.000000") "Undefined" "MultiplyWithRoot" 0 0)
  (Game|SpawnActorfromClass "/Game/Blueprints/BP_EventDisarm.BP_EventDisarm_C" (Math|Transform|MakeTransform (Math|Random|RandomPointinBoundingBox "0.000000,0.000000,80.000000" "50.000000,50.000000,0.000000") "0, 0, 0" "1.000000,1.000000,1.000000") "Undefined" "MultiplyWithRoot" 0 0))

(fn SpawnPotion
  (Game|SpawnActorfromClass "/Game/Blueprints/BP_Potion.BP_Potion_C" (Math|Transform|MakeTransform (Math|Random|RandomPointinBoundingBox "0.000000,0.000000,80.000000" "1000.000000,1000.000000,0.000000") "0, 0, 0" "1.000000,1.000000,1.000000") "Undefined" "MultiplyWithRoot" 0 0))

(fn SpawnPlayers
  (bind _outactors (Actor|GetAllActorsOfClass "/Game/Blueprints/Controller/BP_CustomPlayerController.BP_CustomPlayerController_C"))
  (for _array_element _outactors
    (Class|GameplayStatics|RemovePlayer _array_element false))
  (bind _outactors_2 (Actor|GetAllActorsOfClass "/Script/Engine.PlayerStart"))
  (for (_array_element_2 _array_index) _outactors_2
    (bind _returnvalue (Class|GameplayStatics|CreatePlayer _array_index))
    (bind _asbp_custom_player_controller (Utilities|Casting|CastToBP_CustomPlayerController _returnvalue))
    (Default|SetupInput _asbp_custom_player_controller)
    (bind _returnvalue_2 (Game|SpawnActorfromClass "/Game/Blueprints/BP_Character.BP_Character_C" (Math|Conversions|ToTransform(Vector) (Transformation|GetActorLocation _array_element_2)) "Undefined" "MultiplyWithRoot" 0 0))
    (Pawn|Possess _asbp_custom_player_controller _returnvalue_2)
    (Variables|/Game/Blueprints/BP_Character.BP_Character_C|SetIndex _returnvalue_2 _array_index)))