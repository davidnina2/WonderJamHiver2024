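; BP_Potion is a pickup potion that gives the player a random temporary buff paired with a random debuff.
; On BeginPlay it draws both effects from DT_Effects and takes its color from the buff.
; Overlapping a character with no potion assigns it and teleports it far away instead of destroying it.
; Consume multiplies the player's stats and starts a timer to Expire, which divides multiplier effects back out, clears the slot and destroys the actor.
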(event OnComponentBeginOverlap(Box)
  (params (OverlappedComponent :type Primitive%20Component%20Object%20Reference) (OtherActor :type Actor%20Object%20Reference) (OtherComp :type Primitive%20Component%20Object%20Reference) (OtherBodyIndex :type Integer) (bFromSweep :type Boolean) (SweepResult :type Hit%20Result%20Structure%20%28by%20ref%29))
  (bind _asbp_character (Utilities|Casting|CastToBP_Character OtherActor)
    (:then
      (if (not (Utilities|IsValid (Variables|/Game/Blueprints/BP_Character.BP_Character_C|GetPotion _asbp_character)))
        (Variables|/Game/Blueprints/BP_Character.BP_Character_C|SetPotion _asbp_character self)
        (Transformation|SetActorLocation (Math|Random|RandomPointinBoundingBox "10000.000000,10000.000000,10000.000000" "1000.000000,1000.000000,1000.000000") false true)
        (Default|UpdatePotion _asbp_character)))
    (:CastFailed
      (Development|PrintString (Utilities|GetDisplayName OtherActor)))))

(event Custom|Consume
  (params (Player :type BP%20Character%20Object%20Reference))
  (bind _stats (Variables|/Game/Blueprints/BP_Character.BP_Character_C|GetStats Player))
  (if (not (Variables|Default|GetConsumed))
    (Variables|Default|SetConsumed true)
    (Audio|PlaySoundatLocation "/Game/sounds/DrinkSound.DrinkSound" (Transformation|GetActorLocation Player) "0, 0, 0" 1.0 1.0 0.0 0 0 0 0)
    (bind _output_get (Variables|Default|SetPlayerCharacter Player))
    (for _array_element (Variables|Default|GetEffects)
      (Development|PrintString (Utilities|String|ToString(Float) (* (.Value (Utilities|Map|Find _stats (.Stat (Utilities|Struct|BreakST_Effects _array_element)))) (.Multiplier (Utilities|Struct|BreakST_Effects _array_element)))))
      (Utilities|Map|Add _stats (.Stat (Utilities|Struct|BreakST_Effects _array_element)) (* (.Value (Utilities|Map|Find _stats (.Stat (Utilities|Struct|BreakST_Effects _array_element)))) (.Multiplier (Utilities|Struct|BreakST_Effects _array_element))))
      (Utilities|Time|SetTimerbyEvent (delegate Custom|Expire) (Variables|Default|GetEffectTimer)))
    (Default|UpdatePotion _output_get)))

(event Custom|Expire
  (bind _playercharacter (Variables|Default|GetPlayerCharacter))
  (bind _playercharacter_2 (Variables|Default|GetPlayerCharacter))
  (bind _stats (Variables|/Game/Blueprints/BP_Character.BP_Character_C|GetStats _playercharacter_2))
  (for _array_element 0
    (if (== (.Effect (Utilities|Struct|BreakST_Effects _array_element)) "(TagName=\"effect.modifier.multiplier\")")
      (Utilities|Map|Add _stats (.Stat (Utilities|Struct|BreakST_Effects _array_element)) (/ (.Value (Utilities|Map|Find _stats (.Stat (Utilities|Struct|BreakST_Effects _array_element)))) (.Multiplier (Utilities|Struct|BreakST_Effects _array_element))))))
  (Variables|Default|SetDiscarded true)
  (Variables|/Game/Blueprints/BP_Character.BP_Character_C|SetPotion _playercharacter 0)
  (Default|UpdatePotion _playercharacter)
  (Actor|DestroyActor))

(event EventBeginPlay
  (bind _returnvalue (Utilities|GetDataTableRow "/Game/Data/DT_Effects.DT_Effects" (Utilities|String|StringToName (Utilities|String|Append "Buff_" (Utilities|String|ToString(Integer) (Math|Random|RandomIntegerinRange 1 6)))))
    (:then
      (Variables|Default|SetPotionColor (.Color (Utilities|Struct|BreakST_Effects _returnvalue)))
      (Utilities|Array|Add (Variables|Default|GetEffects) _returnvalue)
      (bind _returnvalue_2 (Utilities|GetDataTableRow "/Game/Data/DT_Effects.DT_Effects" (Utilities|String|StringToName (Utilities|String|Append "Debuff_" (Utilities|String|ToString(Integer) (Math|Random|RandomIntegerinRange 1 6)))))
        (:then
          (Utilities|Array|Add (Variables|Default|GetEffects) _returnvalue_2))))))

(fn ConstructionScript)