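; BP_EventDisarm is an event actor, named for disarming, with a pulsing outline sprite and tracking of the player character in its overlap area.
; On BeginPlay it hides the sprite and starts a Pulse timeline that drives the sprite color's alpha.
; Overlap begin stores a BP_Character reference and any overlap end clears it.
; No disarm logic or code to show the sprite appears in this graph.
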(event Collision|EventActorBeginOverlap
  (params (OtherActor :type Actor%20Object%20Reference))
  (bind _asbp_character (Utilities|Casting|CastToBP_Character OtherActor))
  (Variables|Default|SetCharacter _asbp_character))

(event Collision|EventActorEndOverlap
  (params (OtherActor :type Actor%20Object%20Reference))
  (Variables|Default|SetCharacter 0))

(event EventBeginPlay
  (bind _t_eventoutline_sprite (Variables|Default|GetT_EventOutline_Sprite))
  (bind _spritecolor (Variables|/Script/Paper2D.PaperSpriteComponent|GetSpriteColor _t_eventoutline_sprite))
  (Rendering|SetVisibility (Variables|Default|GetT_EventOutline_Sprite) false false)
  (bind _alpha (Timeline|Pulse PlayFromStart)
    (:Update
      (Sprite|SetSpriteColor _t_eventoutline_sprite (Utilities|Struct|MakeLinearColor (.r _spritecolor) (.g _spritecolor) (.b _spritecolor) _alpha)))))

(fn ConstructionScript)