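; BP_AcidPool is a hazard actor that periodically damages any BP_Character standing in it.
; Overlap begin and end events maintain the PlayersInPool list, which a looping half-second timer started on BeginPlay iterates through.
; Each tick lowers the health entry in every listed character's Stats map, debug-prints the new value, notifies BP_GameMode through HealthUpdated and plays a 2D acid sound.
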(event Custom|DamagePlayer
  (for _array_element (Variables|Default|GetPlayersInPool)
    (Development|PrintString (Utilities|String|ToString(Float) (- (.Value (Utilities|Map|Find (Variables|/Game/Blueprints/BP_Character.BP_Character_C|GetStats _array_element) "(TagName=\"stats.health\")")) 5.0)))
    (Utilities|Map|Add (Variables|/Game/Blueprints/BP_Character.BP_Character_C|GetStats _array_element) "(TagName=\"stats.health\")" (- (.Value (Utilities|Map|Find (Variables|/Game/Blueprints/BP_Character.BP_Character_C|GetStats _array_element) "(TagName=\"stats.health\")")) 5.0))
    (bind _asbp_game_mode (Utilities|Casting|CastToBP_GameMode (Game|GetGameMode)))
    (Default|HealthUpdated _asbp_game_mode)
    (Audio|PlaySound2D "/Game/sounds/acid_damage.acid_damage" 1.0 1.0 0.0 0 0)))

(event Collision|EventActorBeginOverlap
  (params (OtherActor :type Actor%20Object%20Reference))
  (bind _asbp_character (Utilities|Casting|CastToBP_Character OtherActor))
  (Utilities|Array|Add (Variables|Default|GetPlayersInPool) _asbp_character))

(event EventBeginPlay
  (bind _returnvalue (Utilities|Time|SetTimerbyEvent (delegate Custom|DamagePlayer) 0.5 true))
  (Variables|Default|SetTimerHandle _returnvalue))

(event Collision|EventActorEndOverlap
  (params (OtherActor :type Actor%20Object%20Reference))
  (bind _asbp_character (Utilities|Casting|CastToBP_Character OtherActor))
  (Utilities|Array|RemoveItem (Variables|Default|GetPlayersInPool) _asbp_character))

(fn ConstructionScript)